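; Cube Blueprint that periodically swaps its mesh material at random and shows a material name on a text render.
; BeginPlay starts a looping five-second timer that calls ColorMaterial, which picks from the Materials array.
; The mesh and text each get a separate random pick, so the displayed name can differ from the applied material.
; Disconnected leftovers include a MultiGate color cycle and an unfinished RightId matching check.
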(event EventBeginPlay
  (Utilities|Time|SetTimerbyFunctionName 0 "ColorMaterial" (Math|Timespan|GetTotalSeconds (Math|Timespan|FromSeconds 5.0)) true))

(fn ConstructionScript)

(fn ColorMaterial
  (bind _materials (Variables|Default|GetMaterials))
  (bind _returnvalue (Utilities|Array|LastIndex _materials))
  (bind _returnvalue_2 (+ _returnvalue 1))
  (bind _returnvalue_3 (Math|Random|RandomInteger _returnvalue_2))
  (bind _output (Utilities|Array|Get(acopy) _materials _returnvalue_3))
  (Rendering|Material|SetMaterial (Variables|Debug|GetStaticMeshComponent) 0 _output)
  (Rendering|Components|TextRender|SetText (Variables|Default|GetRenderTextName) (Utilities|Text|ToText(Object) _output)))